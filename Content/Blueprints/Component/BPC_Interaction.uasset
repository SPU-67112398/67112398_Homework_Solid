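; Player character interaction component that detects nearby interactable actors, shows a prompt for one and triggers it.
; Each tick, a sphere trace around the owner feeds a list of candidates.
; The first candidate within a view cone from control rotation, not the nearest by distance, positions and labels a screen-space widget created at BeginPlay.
; Interacted repeats that selection, messages the actor and removes it from the list.
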(event `self.ReceiveBeginPlay`
  (bind _interactwidgetcomp (`self.InteractWidgetComp`))
  (bind _asbp_player_character (cast `/Game/ThirdPerson/Blueprints/BP_PlayerCharacter` (`self.GetOwner`)))
  (bind _output_get (set `self.Owner Character` _asbp_player_character))
  (bind _returnvalue (`|AddComponentByClass` _output_get "/Script/UMG.WidgetComponent" true (`KismetMathLibrary.MakeTransform` (0.0 0.0 0.0))))
  (set `self.InteractWidgetComp` _returnvalue)
  (`|ExecutionSequence`
    (:`then_0`
      (`WidgetComponent.SetDrawSize` _interactwidgetcomp (500.0 50.0))
      (`WidgetComponent.SetWidgetSpace` _interactwidgetcomp "Screen"))
    (:`then_1`
      (bind _returnvalue_2 (`|CreateWidget` "/Game/Blueprints/Widget/WBP_Interact.WBP_Interact_C"))
      (bind _output_get_2 (set `self.InteractWidget` _returnvalue_2))
      (`Widget.SetVisibility` _output_get_2 "Collapsed"))
    (:`then_2`
      (`WidgetComponent.SetWidget` (`self.InteractWidgetComp`) (`self.InteractWidget`)))))

(event `self.ReceiveTick`
  (params (DeltaSeconds :type "Float (single-precision)"))
  (bind _closetinteract (`self.ClosetInteract`))
  (`/Engine/EditorBlueprintResources/StandardMacros.IsValid` (`self.Owner Character`)
    (:`Is Valid`
      (`|ExecutionSequence`
        (:`then_0`
          (`self.FindInteractables`))
        (:`then_1`
          (bind _returnclosetinteractable (`self.FindClosetInteractable`))
          (`/Engine/EditorBlueprintResources/StandardMacros.IsValid` _returnclosetinteractable
            (:`Is Valid`
              (if (!= _returnclosetinteractable (`self.ClosetInteract`))
                (set `self.ClosetInteract` _returnclosetinteractable)
                (`|ExecutionSequence`
                  (:`then_0`
                    (`Widget.SetVisibility` (`self.InteractWidget`) "Visible"))
                  (:`then_1`
                    (bind _newparam (message `/Game/Blueprints/Interactable/BPI_Interactable.GetInteractTextLocation` _closetinteract))
                    (`SceneComponent.K2_SetWorldLocation` (`self.InteractWidgetComp`) _newparam false false)
                    (bind _returntext (message `/Game/Blueprints/Interactable/BPI_Interactable.GetInteractableText` _closetinteract))
                    (`/Game/Blueprints/Widget/WBP_Interact.SetInteractText` (`self.InteractWidget`) _returntext)))))
            (:`Is Not Valid`
              (set `self.ClosetInteract` null)
              (`Widget.SetVisibility` (`self.InteractWidget`) "Collapsed"))))))))

(fn `FindClosetInteractable`
  (returns (ReturnClosetInteractable :type "Actor Object Reference"))
  (bind _foundinteractable (`self.FoundInteractable`))
  (if (`KismetArrayLibrary.Array_IsNotEmpty` _foundinteractable)
    (for _array_element _foundinteractable
      (if (`self.IsInteractableInView` _array_element)
        (return _array_element))))
  (return null))

(fn `FindInteractables`
  (locals (TempInteractable :type "Array of Actor Object Reference"))
  (bind _foundinteractable (`self.FoundInteractable`))
  (bind _returnvalue (`Actor.K2_GetActorLocation` (`self.Owner Character`)))
  (bind (_outhits _returnvalue_2) (`KismetSystemLibrary.SphereTraceMulti` _returnvalue _returnvalue 100.0 "TraceTypeQuery1"))
  (if _returnvalue_2
    ; Temp Interactable
    (for _array_element _outhits
      (bind (_bblockinghit _binitialoverlap _time _distance _location _impactpoint _normal _impactnormal _physmat _hitactor) (`GameplayStatics.BreakHitResult` _array_element))
      (bind _retuniscan (message `/Game/Blueprints/Interactable/BPI_Interactable.CanInteractable` _hitactor))
      (if (and _bblockinghit _retuniscan)
        (`KismetArrayLibrary.Array_Add` (`local.TempInteractable`) _hitactor)))
    (if (`KismetArrayLibrary.Array_IsEmpty` (`self.FoundInteractable`))
      (`KismetArrayLibrary.Array_Append` (`self.FoundInteractable`) (`local.TempInteractable`))
      (else
        (bind (_arrayindex _arrayelement) (`/Engine/EditorBlueprintResources/StandardMacros.ReverseForEachLoop` _foundinteractable)
          (:`LoopBody`
            (if (not (`KismetArrayLibrary.Array_Contains` (`local.TempInteractable`) _arrayelement))
              (`KismetArrayLibrary.Array_RemoveItem` _foundinteractable _arrayelement))))))
    (else
      (`KismetArrayLibrary.Array_Clear` (`self.FoundInteractable`)))))

(fn `Interacted`
  (locals (TmpInteract :type "Actor Object Reference"))
  (bind _foundinteractable (`self.FoundInteractable`))
  (bind _tmpinteract (`local.TmpInteract`))
  (if (`KismetArrayLibrary.Array_IsNotEmpty` _foundinteractable)
    (for _array_element _foundinteractable
      (if (`self.IsInteractableInView` _array_element)
        (set `local.TmpInteract` _array_element)
        (break)))
    (`/Engine/EditorBlueprintResources/StandardMacros.IsValid` _tmpinteract
      (:`Is Valid`
        (`|ExecutionSequence`
          (:`then_0`
            (message `/Game/Blueprints/Interactable/BPI_Interactable.OnInteract` _tmpinteract (`self.Owner Character`)))
          (:`then_1`
            (`KismetArrayLibrary.Array_RemoveItem` (`self.FoundInteractable`) _tmpinteract)))))))

(fn `IsInteractableInView`
  (params (Interactable :type "Actor Object Reference"))
  (returns (ReturnValue :type Boolean))
  (return (<= (`KismetMathLibrary.DegAcos` (`KismetMathLibrary.Dot_VectorVector` (`KismetMathLibrary.GetForwardVector` (`Pawn.GetControlRotation` (`self.Owner Character`))) (`KismetMathLibrary.Normal` (- (`Actor.K2_GetActorLocation` Interactable) (`Actor.K2_GetActorLocation` (`self.GetOwner`)))))) 120.0)))