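; BPC_Inventory is an inventory component that holds item objects with slot indices and quantities.
; AddItemByClass increments an existing item of the same class, or constructs one at quantity 0 while reporting a quantity of 1.
; UseItemBySlot sends ConsumeMessage to the slot's item with the owner, decrementing the quantity only on success.
; Both functions broadcast OnInventoryUpdated with slot and quantity when changes occur.
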(fn `AddItemByClass`
  (params (ItemClass :type "/Game/Blueprints/Interactable/BP_Inventory_Item_Base Class Reference"))
  (locals (bFoundItem :type Boolean))
  (for _array_element (`self.Items`)
    (if (== (`GameplayStatics.GetObjectClass` _array_element) ItemClass)
      (bind _output_get (set `/Game/Blueprints/Interactable/BP_Inventory_Item_Base.Quantity` (+ (`/Game/Blueprints/Interactable/BP_Inventory_Item_Base.Quantity` _array_element) 1) _array_element))
      (`self.OnInventoryUpdated` (`/Game/Blueprints/Interactable/BP_Inventory_Item_Base.SlotIndex` _array_element) _output_get)
      (return)))
  (bind _returnvalue (`|GenericCreateObject` (`self.GetOwner`) ItemClass))
  (set `/Game/Blueprints/Interactable/BP_Inventory_Item_Base.Quantity` 0 _returnvalue)
  (`KismetArrayLibrary.Array_Add` (`self.Items`) _returnvalue)
  (`self.OnInventoryUpdated` (`/Game/Blueprints/Interactable/BP_Inventory_Item_Base.SlotIndex` _returnvalue) 1)
  (return))

(fn `UseItemBySlot`
  (params (TargetSlot :type Integer))
  (for _array_element (`self.Items`)
    (bind _slotindex (`/Game/Blueprints/Interactable/BP_Inventory_Item_Base.SlotIndex` _array_element))
    (if (== _slotindex TargetSlot)
      (bind _quantity (`/Game/Blueprints/Interactable/BP_Inventory_Item_Base.Quantity` _array_element))
      (if (> _quantity 0)
        (bind _issuccess (message `/Game/Blueprints/Component/BPI_Consumable_Item.Consume` _array_element (`self.GetOwner`)))
        (if _issuccess
          (bind _output_get (set `/Game/Blueprints/Interactable/BP_Inventory_Item_Base.Quantity` (- _quantity 1) _array_element))
          (`self.OnInventoryUpdated` _slotindex _output_get)
          (`KismetSystemLibrary.PrintString` "[Use Success] Slot 0, Remaining:")
          (break)
          (else
            (break)))))))