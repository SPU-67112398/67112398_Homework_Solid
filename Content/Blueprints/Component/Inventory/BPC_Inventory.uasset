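; Inventory component that creates three fixed item objects (heal, speed, coin) on BeginPlay and tracks their quantities.
; AddItem raises the quantity of the entry matching a class, and UseItem decrements one by index when its ConsumeMessage call on the user succeeds.
; Both call OnInventoryUpdated after a change.
; GetItemCount is unfinished, with a disconnected loop and a return of zero.
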(event EventBeginPlay
  (bind _returnvalue (Game|ConstructObjectfromClass (Components|GetOwner) "/Game/Blueprints/Component/Inventory/BP_Inventory_Item_Heal.BP_Inventory_Item_Heal_C"))
  (Utilities|Array|Add (Variables|Default|GetItems) _returnvalue)
  (bind _returnvalue_2 (Game|ConstructObjectfromClass (Components|GetOwner) "/Game/Blueprints/Component/Inventory/BP_Inventory_Item_Speed.BP_Inventory_Item_Speed_C"))
  (Utilities|Array|Add (Variables|Default|GetItems) _returnvalue_2)
  (bind _returnvalue_3 (Game|ConstructObjectfromClass (Components|GetOwner) "/Game/Blueprints/Component/Inventory/BP_Inventory_Item_Coin.BP_Inventory_Item_Coin_C"))
  (Utilities|Array|Add (Variables|Default|GetItems) _returnvalue_3))

(event EventTick
  (params (DeltaSeconds :type Float%20%28single-precision%29)))

(fn AddItem
  (params (Class_Item :type BP%20Inventory%20Item%20Base%20Class%20Reference%20%28by%20ref%29) (Amount :type Integer))
  (for _array_element (Variables|Default|GetItems)
    (if (== (Utilities|GetClass _array_element) Class_Item)
      (Variables|/Game/Blueprints/Component/Inventory/BP_Inventory_Item_Base.BP_Inventory_Item_Base_C|SetQuantity _array_element (+ (Variables|/Game/Blueprints/Component/Inventory/BP_Inventory_Item_Base.BP_Inventory_Item_Base_C|GetQuantity _array_element) Amount))
      (Default|CallOnInventoryUpdated)
      (Utilities|FlowControl|ForLoopwithBreak 0 0) ; enters at Break
    )))

(fn UseItem
  (params (Index :type Integer) (User :type BP%20Third%20Person%20Character%20Object%20Reference))
  (bind _items (Variables|Default|GetItems))
  (bind _output (Utilities|Array|Get(acopy) _items Index))
  (if (> (Variables|/Game/Blueprints/Component/Inventory/BP_Inventory_Item_Base.BP_Inventory_Item_Base_C|GetQuantity _output) 0)
    (bind _issuccess (Class|BPIConsumableItem|Consume(Message) _output User))
    (if _issuccess
      (Variables|/Game/Blueprints/Component/Inventory/BP_Inventory_Item_Base.BP_Inventory_Item_Base_C|SetQuantity _output (- (Variables|/Game/Blueprints/Component/Inventory/BP_Inventory_Item_Base.BP_Inventory_Item_Base_C|GetQuantity _output) 1))
      (Default|CallOnInventoryUpdated))))

(fn GetItemCount
  (params (Class_Item :type BP%20Inventory%20Item%20Base%20Class%20Reference%20%28by%20ref%29))
  (if (== (Utilities|GetClass (stale _array_element)) Class_Item)
    (return 0)))