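; BP_Door is an interactable door that swings open and closed on alternate interactions and supplies an "Open Door" prompt at its InteractPoint.
; OnInteract sets a motion warp target at a fixed offset from the door toward the interactor, facing it, then plays the opening montage on the interactor.
; After a short delay, a FlipFlop plays or reverses a Timeline that yaws InteractPoint.
; Montage completion or interruption clears IsInteract.
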(event `/Game/Blueprints/Interactable/BPI_Interactable.OnInteract`
  (params (Interactor :type "/Game/ThirdPerson/Blueprints/BP_PlayerCharacter Object Reference"))
  (bind _returnvalue (`self.K2_GetActorLocation` self))
  (bind _returnvalue_2 (`KismetMathLibrary.Normal` (- (`self.K2_GetActorLocation` Interactor) _returnvalue)))
  (bind (_returnvalue_x _returnvalue_y) (`KismetMathLibrary.BreakVector` (* _returnvalue_2 -1.0)))
  (`parent.OnInteract` Interactor)
  (`MotionWarpingComponent.AddOrUpdateWarpTargetFromLocationAndRotation` (`/Game/ThirdPerson/Blueprints/BP_ThirdPersonCharacter.MotionWarping` Interactor) "InteractDoor" (+ (* _returnvalue_2 65.0) _returnvalue) (`KismetMathLibrary.MakeRotFromX` (`KismetMathLibrary.MakeVector` _returnvalue_x _returnvalue_y)))
  (`|PlayMontage` (`Character.Mesh` Interactor) "/Game/Characters/Animation/A_OpenDoor_R_Montage.A_OpenDoor_R_Montage"
    (:`then`
      (`KismetSystemLibrary.Delay` 0.3)
      (`/Engine/EditorBlueprintResources/StandardMacros.FlipFlop`
        (:`A`
          (bind (_direction _door) (`Timeline|Timeline` :!label _label)
            (:`Update`
              (`SceneComponent.K2_SetRelativeRotation` (`self.InteractPoint`) (`KismetMathLibrary.MakeRotator` 0.0 0.0 _door) false false))))
        (:`B`
          (goto _label :!via `Reverse`))))
    (:`OnCompleted`
      (set `self.IsInteract` false :!label _label_2))
    (:`OnInterrupted`
      (goto _label_2))))

(fn `GetInteractableText`
  (returns (ReturnText :type Text))
  (return "Open Door"))

(fn `GetInteractTextLocation`
  (returns (NewParam :type "Vector Structure"))
  (return (`SceneComponent.K2_GetComponentLocation` (`self.InteractPoint`))))

(fn `UserConstructionScript`
  (`parent.UserConstructionScript`))