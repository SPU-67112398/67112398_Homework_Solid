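; Speed boost inventory item that raises the consuming user's CharacterMovement max walk speed when used.
; Consume rejects use while IsBoosting is set; otherwise it caches the movement component, applies the boost and starts a timer by function name.
; That timer targets the User rather than this item, and the ResetSpeed logic here that restores speed and clears the flag is unconnected.
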(fn `Consume`
  (params (User :type "Actor Object Reference"))
  (returns (IsSuccess :type Boolean))
  (bind _returnvalue (`Actor.GetComponentByClass` User "/Script/Engine.CharacterMovementComponent"))
  (if (`self.bIsBoosting`)
    (return false)
    (else
      (set `self.bIsBoosting` true)
      (set `self.MovementComp` _returnvalue)
      (set `CharacterMovementComponent.MaxWalkSpeed` 1200.0 _returnvalue)
      (`KismetSystemLibrary.K2_SetTimer` User "ResetSpeed" 5.0)
      (return true))))